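; Player controller that lets BP_Character pick up, drop and use access cards on turnstiles.
; E, F and Q play take, drop and use montages with movement disabled, turning the character toward nearby targets found by sphere overlaps for take and use.
; Separate events, not called within this graph, apply the results: copying card data to the character, respawning the dropped card, or comparing tags to open the turnstile or signal refusal.
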(event `self.ReceiveBeginPlay`
  (bind _asbp_character (cast `/Game/MyContent/Blueprints/BP_Character` (`GameplayStatics.GetPlayerPawn` 0)))
  (set `self.PlayerPawn` _asbp_character))

(event `Event_TakeCard`
  (bind _playerpawn (`self.PlayerPawn`))
  (bind _card (`/Game/MyContent/Blueprints/BP_Character.Card` _playerpawn))
  ;[1 1 1] Подятие карты
  (bind _outactors (`KismetSystemLibrary.SphereOverlapActors` (`self.K2_GetActorLocation` (`self.PlayerPawn`)) 70.0 (`|MakeArray` "ObjectTypeQuery1" "ObjectTypeQuery2" :!type "EObjectTypeQuery Enum") "/Game/MyContent/Blueprints/Card/BP_Card.BP_Card_C"))
  (bind _output (`|GetArrayItem` _outactors))
  (bind _asbp_card (cast `/Game/MyContent/Blueprints/Card/BP_Card` _output))
  (set `/Game/MyContent/Blueprints/BP_Character.TakenCard` (`/Game/MyContent/Blueprints/Card/BP_Card.ST_Card` _asbp_card) _playerpawn)
  (set `/Game/MyContent/Blueprints/BP_Character.CardWasTaken` true _playerpawn)
  (`self.K2_DestroyActor` _output)
  (`SceneComponent.SetHiddenInGame` _card false false)
  (`PrimitiveComponent.SetMaterial` _card 0 (`.Color_6_968E5C3F4D15192586EA4A846D3ECB21` (break `/Game/MyContent/Blueprints/Card/ST_Card` (`/Game/MyContent/Blueprints/BP_Character.TakenCard` (`self.PlayerPawn`))))))

(event `Key|E`
  (params (Key :type "Key Structure"))
  (:`Pressed`
    (if (not (`/Game/MyContent/Blueprints/BP_Character.CardWasTaken` (`self.PlayerPawn`)))
      (bind _outactors (`KismetSystemLibrary.SphereOverlapActors` (`self.K2_GetActorLocation` (`self.PlayerPawn`)) 70.0 (`|MakeArray` "ObjectTypeQuery1" "ObjectTypeQuery2" :!type "EObjectTypeQuery Enum") "/Game/MyContent/Blueprints/Card/BP_Card.BP_Card_C"))
      (if (> (`KismetArrayLibrary.Array_Length` _outactors) 0)
        (`self.Fun_SetPlayerRotation` (`|GetArrayItem` _outactors))
        (`|PlayMontage` (`Character.Mesh` (`self.PlayerPawn`)) "/Game/Mannequin/Animations/UseableAnim/AnimM_ThirdPersonTake.AnimM_ThirdPersonTake"
          (:`then`
            (`CharacterMovementComponent.SetMovementMode` (`Character.CharacterMovement` (`self.PlayerPawn`)) "MOVE_None" 0 :!label _label))
          (:`OnCompleted`
            (`CharacterMovementComponent.SetMovementMode` (`Character.CharacterMovement` (`self.PlayerPawn`)) "MOVE_Walking" 0 :!label _label_2)))))))

(event `Key|F`
  (params (Key :type "Key Structure"))
  (:`Pressed`
    (if (`/Game/MyContent/Blueprints/BP_Character.CardWasTaken` (`self.PlayerPawn`))
      (`|PlayMontage` (`Character.Mesh` (`self.PlayerPawn`)) "/Game/Mannequin/Animations/UseableAnim/AnimM_ThirdPersonDrop.AnimM_ThirdPersonDrop"
        (:`then`
          (goto _label))
        (:`OnCompleted`
          (goto _label_2))))))

(event `Event_DropCard`
  (bind _playerpawn (`self.PlayerPawn`))
  ;[1 1 1] Выбрасываем карту
  (`self.Func_DropCard`)
  (set `/Game/MyContent/Blueprints/BP_Character.CardWasTaken` false _playerpawn)
  (`SceneComponent.SetHiddenInGame` (`/Game/MyContent/Blueprints/BP_Character.Card` _playerpawn) true false))

(event `Key|Q`
  (params (Key :type "Key Structure"))
  (:`Pressed`
    (if (`/Game/MyContent/Blueprints/BP_Character.CardWasTaken` (`self.PlayerPawn`))
      (bind _outactors (`KismetSystemLibrary.SphereOverlapActors` (`self.K2_GetActorLocation` (`self.PlayerPawn`)) 60.0 (`|MakeArray` "ObjectTypeQuery1" "ObjectTypeQuery2" :!type "EObjectTypeQuery Enum") "/Game/MyContent/Blueprints/BP_Turnstile.BP_Turnstile_C"))
      (if (> (`KismetArrayLibrary.Array_Length` _outactors) 0)
        (`self.Fun_SetPlayerRotation` (`|GetArrayItem` _outactors))
        (`|PlayMontage` (`Character.Mesh` (`self.PlayerPawn`)) "/Game/Mannequin/Animations/UseableAnim/AnimM_ThirdPersonUse.AnimM_ThirdPersonUse"
          (:`then`
            (goto _label))
          (:`OnCompleted`
            (goto _label_2)))))))

(event `Event_UseCard`
  ;[1 1 1] Используем карту
  (bind _outactors (`KismetSystemLibrary.SphereOverlapActors` (`self.K2_GetActorLocation` (`self.PlayerPawn`)) 60.0 (`|MakeArray` "ObjectTypeQuery1" "ObjectTypeQuery2" :!type "EObjectTypeQuery Enum") "/Game/MyContent/Blueprints/BP_Turnstile.BP_Turnstile_C"))
  (bind _asbp_turnstile (cast `/Game/MyContent/Blueprints/BP_Turnstile` (`|GetArrayItem` _outactors)))
  (if (== (`/Game/MyContent/Blueprints/BP_Turnstile.Tag` _asbp_turnstile) (`.Tag_4_AD510C9341BE36859381DA9600A3E4B3` (break `/Game/MyContent/Blueprints/Card/ST_Card` (`/Game/MyContent/Blueprints/BP_Character.TakenCard` (`self.PlayerPawn`)))))
    (`KismetSystemLibrary.PrintString` "Yes")
    (`/Game/MyContent/Blueprints/BP_Turnstile.Event_Open_Close` _asbp_turnstile)
    (else
      (`KismetSystemLibrary.PrintString` "No")
      (`/Game/MyContent/Blueprints/BP_Turnstile.Event Light Card` _asbp_turnstile true))))

(fn `Fun_SetPlayerRotation`
  (params (Aim :type "Actor Object Reference"))
  (bind _playerpawn (`self.PlayerPawn`))
  (bind (_returnvalue_roll _returnvalue_pitch _returnvalue_yaw) (`KismetMathLibrary.BreakRotator` (`KismetMathLibrary.FindLookAtRotation` (`self.K2_GetActorLocation` _playerpawn) (`self.K2_GetActorLocation` Aim))))
  (`self.K2_SetActorRotation` _playerpawn (`KismetMathLibrary.MakeRotator` 0.0 0.0 _returnvalue_yaw) false))

(fn `Func_DropCard`
  (bind _playerpawn (`self.PlayerPawn`))
  (`|SpawnActorFromClass` "/Game/MyContent/Blueprints/Card/BP_Card.BP_Card_C" (`KismetMathLibrary.MakeTransform` (`SceneComponent.K2_GetComponentLocation` (`/Game/MyContent/Blueprints/BP_Character.Card` _playerpawn))) "Undefined" "OverrideRootScale" null (`/Game/MyContent/Blueprints/BP_Character.TakenCard` _playerpawn) null))

(fn `UserConstructionScript`)