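; Turnstile that shows a widget while the player, having taken a card, is inside its sphere trigger.
; An open/close event, gated by a DoOnce, lights the lamp green and plays a timeline that rotates the gate.
; A FlipFlop on timeline finish alternates between a timed auto-close and re-arming the DoOnce.
; The light event shows red or green, then a restartable timer blanks the lamp.
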(event `self.ReceiveBeginPlay`
  (bind _asbp_character (cast `/Game/MyContent/Blueprints/BP_Character` (`GameplayStatics.GetPlayerPawn` 0)))
  (set `self.Player` _asbp_character))

(event `self.Sphere.OnComponentBeginOverlap`
  (params (OverlappedComponent :type "PrimitiveComponent Object Reference") (OtherActor :type "Actor Object Reference") (OtherComp :type "PrimitiveComponent Object Reference") (OtherBodyIndex :type Integer) (bFromSweep :type Boolean) (SweepResult :type "HitResult Structure (by ref)"))
  (if (`self.ActorHasTag` OtherActor "Player")
    (if (`/Game/MyContent/Blueprints/BP_Character.CardWasTaken` (`self.Player`))
      (`SceneComponent.SetHiddenInGame` (`self.Widget`) false false))))

(event `self.Sphere.OnComponentEndOverlap`
  (params (OverlappedComponent :type "PrimitiveComponent Object Reference") (OtherActor :type "Actor Object Reference") (OtherComp :type "PrimitiveComponent Object Reference") (OtherBodyIndex :type Integer))
  (if (`self.ActorHasTag` OtherActor "Player")
    (`SceneComponent.SetHiddenInGame` (`self.Widget`) true false)))

(event `WaitBeforClose`
  (bind (_direction _up_down) (`Timeline|Up_Down` :!via `Reverse` :!label _label)
    (:`Update`
      (`SceneComponent.K2_SetRelativeRotation` (`self.Scene`) (`KismetMathLibrary.RLerp` (struct) (struct :`Pitch` 90.0) _up_down) false false))
    (:`Finished`
      (`/Engine/EditorBlueprintResources/StandardMacros.FlipFlop`
        (:`A`
          (`KismetSystemLibrary.K2_SetTimerDelegate` (delegate `WaitBeforClose`) 5.0))
        (:`B`
          (goto _label_2 :!via `Reset`))))))

(event `Event_Open_Close`
  (`/Engine/EditorBlueprintResources/StandardMacros.DoOnce` false :!label _label_2
    (:`Completed`
      (`self.Event Light Card` false)
      (goto _label))))

(event `Event Light Card`
  (params (`Wrong?` :type Boolean))
  (bind _lamp (`self.Lamp`))
  (`KismetSystemLibrary.K2_PauseTimerHandle` (`self.TimerLightColor`))
  (if `Wrong?`
    (`PrimitiveComponent.SetMaterial` _lamp 0 "/Game/MyContent/Materials/Lights/MI_Light_Red.MI_Light_Red")
    (else
      (`PrimitiveComponent.SetMaterial` _lamp 0 "/Game/MyContent/Materials/Lights/MI_Light_Green.MI_Light_Green")))
  (bind _returnvalue (`KismetSystemLibrary.K2_SetTimerDelegate` (delegate `LightColor`) 2.0))
  (set `self.TimerLightColor` _returnvalue))

(event `LightColor`
  (`PrimitiveComponent.SetMaterial` (`self.Lamp`) 0 "/Game/MyContent/Materials/Lights/MI_Light_Empty.MI_Light_Empty"))

(fn `UserConstructionScript`)