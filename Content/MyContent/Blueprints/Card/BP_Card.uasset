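; BP_Card is a card actor that shows a widget when the player comes near.
; On BeginPlay it applies the color material from its STCard struct to the Cube and caches the player's BP_Character.
; Sphere overlap with an actor tagged Player reveals the Widget unless that character's CardWasTaken flag is set, and leaving hides it.
; The pickup itself is not handled in these graphs.
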(event `self.ReceiveBeginPlay`
  (`PrimitiveComponent.SetMaterial` (`self.Cube`) 0 (`.Color_6_968E5C3F4D15192586EA4A846D3ECB21` (break `/Game/MyContent/Blueprints/Card/ST_Card` (`self.ST_Card`))))
  (bind _asbp_character (cast `/Game/MyContent/Blueprints/BP_Character` (`GameplayStatics.GetPlayerPawn` 0)))
  (set `self.Player` _asbp_character))

(event `self.Sphere.OnComponentBeginOverlap`
  (params (OverlappedComponent :type "PrimitiveComponent Object Reference") (OtherActor :type "Actor Object Reference") (OtherComp :type "PrimitiveComponent Object Reference") (OtherBodyIndex :type Integer) (bFromSweep :type Boolean) (SweepResult :type "HitResult Structure (by ref)"))
  (if (`self.ActorHasTag` OtherActor "Player")
    (if (not (`/Game/MyContent/Blueprints/BP_Character.CardWasTaken` (`self.Player`)))
      (`SceneComponent.SetHiddenInGame` (`self.Widget`) false false))))

(event `self.Sphere.OnComponentEndOverlap`
  (params (OverlappedComponent :type "PrimitiveComponent Object Reference") (OtherActor :type "Actor Object Reference") (OtherComp :type "PrimitiveComponent Object Reference") (OtherBodyIndex :type Integer))
  (if (`self.ActorHasTag` OtherActor "Player")
    (`SceneComponent.SetHiddenInGame` (`self.Widget`) true false)))

(fn `UserConstructionScript`)